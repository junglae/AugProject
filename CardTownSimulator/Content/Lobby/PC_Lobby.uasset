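; Lobby player controller that creates, finds, joins and exits LAN sessions, and handles ready toggling or host game start.
; Game instance Hosting/Joined flags choose lobby or in-session UI from HUD_Lobby; GM_Lobby handles player updates, starting and kicking.
; Search results pass through a ping filter and sort before display.
; An ActionTimer, often a long dummy timer, serves as a busy flag that Tick reads to enable buttons.
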(event Custom|Find%20Sessions
  ;[1 1 1] Session Control
  (|FindingProcess))

(event Custom|Create%20Session
  ;[1 1 1] Session Control
  (|CreatingProcess))

(event Custom|On%20Ready%20Button%20Clicked
  (if (Variables|/Script/ProjectP.EventGameInstanceSubsystem|GetbHosting (Subsystems|GetEventGameInstanceSubsystem))
    (CallFunction|StartGame)
    (else
      (CallFunction|ToggleReady))))

(event Custom|Close%20Session
  (Default|KickAll (Variables|Default|GetServer)))

(event Custom|Toggle%20Ready
  (|Toggle)
  (Default|UpdatePlayers (Variables|Default|GetServer)))

(event Custom|Start%20Game
  (Default|StartGame (Variables|Default|GetServer)))

(event Custom|Start%20Session
  (Default|StartGame (Variables|Default|GetServer)))

(event Custom|Join%20Session
  ;[1 1 1] Session Control
  (|JoiningProcess))

(event Custom|Set%20Session
  (params (Session :type Blueprint%20Session%20Result%20Structure))
  (Variables|Default|SetSelected%20Session Session))

(event Custom|Cancel%20Find
  ;[1 1 1] Session Control
  (|CancellingProcess))

(event Custom|Exit%20Session
  ;[1 1 1] Session Control
  (|ExitingProcess))

(event Custom|Update%20Players%20Info
  (params (Info :type Array%20of%20Member%20Info%20Structures))
  (|Valid?)
  (bind ___ (Utilities|NullConditional (Variables|Default|GetUI)))
  (Default|UpdatePlayers ___ Info (Variables|/Script/ProjectP.EventGameInstanceSubsystem|GetbHosting (Subsystems|GetEventGameInstanceSubsystem))))

(event Custom|Init%20Server%20Reference
  (bind _output_get (Variables|Default|SetServer (.AsGM%20Lobby (Utilities|Casting|CastToGM_Lobby (Game|GetGameMode)))))
  (Default|UpdatePlayers _output_get))

(event Custom|Init%20Player%20Info
  (|CheckGUIDandInfo))

(event EventTick
  (params (DeltaSeconds :type Float%20%28single-precision%29))
  (bind ___ (Utilities|NullConditional (Variables|Default|GetUI)))
  (|SetButtonActive ___))

(event EventBeginPlay
  (|SetUIReference)
  (|SetGIReference
    (:In%20Session
      (|InSessionProcess))
    (:Standalone
      (Default|GenerateLobbyUI (Variables|Default|GetUI)))))

(fn ConstructionScript)

(fn DummyTimerFunction)

(fn OrderbyResultwithPing
  (params (Array :type Array%20of%20Blueprint%20Session%20Result%20Structures))
  (bind _remains (LocalVariables|GetRemains))
  (bind _remains_2 (LocalVariables|GetRemains))
  (bind _returnvalue (Utilities|Array|LastIndex _remains_2))
  (for _array_element Array
    (if (< (Class|FindSessionsCallbackProxy|GetPinginMs _array_element) 250)
      (bind (_array_element_2 _array_index) (Utilities|Array|ForEachLoopwithBreak _remains :!label _label)
        (:LoopBody
          (if (< (Class|FindSessionsCallbackProxy|GetPinginMs _array_element) (Class|FindSessionsCallbackProxy|GetPinginMs _array_element_2))
            (Utilities|FlowControl|Sequence
              (:then_0
                (Utilities|Array|Insert _remains _array_element _array_index))
              (:then_1
                (goto _label Break)))))
        (:Completed
          (Utilities|Array|AddUnique _remains_2 _array_element)
          (if (> _returnvalue 9)
            (Utilities|Array|RemoveIndex (LocalVariables|GetRemains) _returnvalue))))))
  (return (LocalVariables|GetRemains)))