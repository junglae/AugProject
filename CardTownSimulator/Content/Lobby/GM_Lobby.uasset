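; Lobby game mode that tracks connected players, starts the match and can close the lobby.
; Every Tick it rebuilds arrays of PC_Lobby controllers and their info structs, marks the first entry as ready, and pushes the full list to each controller.
; StartGame performs an absolute ServerTravel to the Gameplay map.
; KickAll kicks every listed player with a server-closed reason.
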(event Custom|Start%20Game
  (Class|AdvancedSessionsLibrary|ServerTravel "Gameplay" true false))

(event Custom|Kick%20All
  (for _array_element (Variables|Default|GetPlayers)
    (Class|AdvancedSessionsLibrary|KickPlayer _array_element "Server Closed")))

(event EventTick
  (params (DeltaSeconds :type Float%20%28single-precision%29))
  (CallFunction|UpdatePlayers))

(fn ConstructionScript)

(fn UpdatePlayers
  (Utilities|Array|Clear)
  (Utilities|Array|MakeArray)
  (|SendInfo))