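; Peasant card Blueprint, a child card class that defines what happens when the card is used.
; OnCardUse runs the parent behavior, then adds a fixed amount to MultipleChanceTurn in the server's State.
; The event graph holds only disabled default events, and the construction script just calls its parent.
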(event EventBeginPlay
  (|CallParentFunction) ; 지금 이 노드는 비활성 상태입니다. \n핀을 끌어서 다른 노드를 연결하면 활성화됩니다.
)

(event Collision|EventActorBeginOverlap
  (params (OtherActor :type Actor%20Object%20Reference))
  (|CallParentFunction OtherActor) ; 지금 이 노드는 비활성 상태입니다. \n핀을 끌어서 다른 노드를 연결하면 활성화됩니다.
)

(event EventTick
  (params (DeltaSeconds :type Float%20%28single-precision%29))
  (|CallParentFunction DeltaSeconds) ; 지금 이 노드는 비활성 상태입니다. \n핀을 끌어서 다른 노드를 연결하면 활성화됩니다.
)

(fn ConstructionScript
  (|CallParentFunction))

(fn OnCardUse
  (params (Player :type PC%20Gameplay%20Object%20Reference) (Server :type GM%20Gameplay%20Object%20Reference))
  (bind _state (Variables|/Game/Server/GM_Gameplay.GM_Gameplay_C|GetState Server))
  (|CallParentFunction Player Server)
  (Variables|/Game/Server/GS_Gameplay.GS_Gameplay_C|SetMultipleChance_Turn _state (+ (Variables|/Game/Server/GS_Gameplay.GS_Gameplay_C|GetMultipleChance_Turn _state) 0.3)))