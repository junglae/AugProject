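; C_Cleric is the Cleric card, a child card Blueprint that activates the Cleric ability when played.
; IsUsable allows the card only while the given player state's ClericCardUsed flag is unset.
; OnCardUse runs the parent logic, then sets ClericAbility on the gameplay state and marks the card as used on the player's state.
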(fn ConstructionScript
  (|CallParentFunction))

(fn IsUsable
  (params (PlayerState :type PS%20Gameplay%20Object%20Reference))
  (return (not (Variables|/Game/Server/PS_Gameplay.PS_Gameplay_C|GetbClericCardUsed PlayerState))))

(fn OnCardUse
  (params (Player :type PC%20Gameplay%20Object%20Reference) (Server :type GM%20Gameplay%20Object%20Reference))
  (|CallParentFunction Player Server)
  (Variables|/Game/Server/GS_Gameplay.GS_Gameplay_C|SetbClericAbility (Variables|/Game/Server/GM_Gameplay.GM_Gameplay_C|GetState (Variables|Default|GetGameplay)) true)
  (Variables|/Game/Server/PS_Gameplay.PS_Gameplay_C|SetbClericCardUsed (Variables|/Game/Client/PC_Gameplay.PC_Gameplay_C|GetState Player) true))