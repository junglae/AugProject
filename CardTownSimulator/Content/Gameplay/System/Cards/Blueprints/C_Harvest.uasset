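; C_Harvest is a card Blueprint that, when used, has a chance to grant resources based on a structure count.
; Its OnCardUse override calls the parent, then reads the count of one structure type from the Server state's Structures map.
; For each of those structures, a random bool decides whether one unit of a single resource type is added to that state.
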(event EventBeginPlay)

(event Collision|EventActorBeginOverlap
  (params (OtherActor :type Actor%20Object%20Reference)))

(event EventTick
  (params (DeltaSeconds :type Float%20%28single-precision%29)))

(fn ConstructionScript
  (|CallParentFunction))

(fn OnCardUse
  (params (Player :type PC%20Gameplay%20Object%20Reference) (Server :type GM%20Gameplay%20Object%20Reference))
  (|CallParentFunction Player Server)
  (for _index (range 1 (.Value (Utilities|Map|Find (Variables|/Game/Gameplay/System/Server/GS_Gameplay.GS_Gameplay_C|GetStructures (Variables|/Game/Gameplay/System/Server/GM_Gameplay.GM_Gameplay_C|GetState Server)) "NewEnumerator2")))
    (if (Math|Random|RandomBool)
      (Default|AddResource (Variables|/Game/Gameplay/System/Server/GM_Gameplay.GM_Gameplay_C|GetState Server) "NewEnumerator0" 1))))