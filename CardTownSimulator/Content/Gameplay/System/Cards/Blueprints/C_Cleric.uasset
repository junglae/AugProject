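; Cleric card Blueprint that activates the Cleric ability and can be used once per player until its used flag is cleared.
; IsUsable allows play only while the player state's ClericCardUsed flag is false.
; OnCardUse runs the parent logic, then sets ClericAbility on the Gameplay state and marks the card used on the player's state.
; The effect of the ability itself is handled outside this card.
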(fn ConstructionScript
  (|CallParentFunction))

(fn IsUsable
  (params (PlayerState :type PS%20Gameplay%20Object%20Reference))
  (return (not (Variables|/Game/Gameplay/System/Server/PS_Gameplay.PS_Gameplay_C|GetbClericCardUsed PlayerState))))

(fn OnCardUse
  (params (Player :type PC%20Gameplay%20Object%20Reference) (Server :type GM%20Gameplay%20Object%20Reference))
  (|CallParentFunction Player Server)
  (Variables|/Game/Gameplay/System/Server/GS_Gameplay.GS_Gameplay_C|SetbClericAbility (Variables|/Game/Gameplay/System/Server/GM_Gameplay.GM_Gameplay_C|GetState (Variables|Default|GetGameplay)) true)
  (Variables|/Game/Gameplay/System/Server/PS_Gameplay.PS_Gameplay_C|SetbClericCardUsed (Variables|/Game/Gameplay/Client/PC_Gameplay.PC_Gameplay_C|GetState Player) true))