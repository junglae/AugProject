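; C_Revelation is a card Blueprint that triggers the server's Revelation effect when a player uses it.
; Each use runs the parent logic, calls ActivateCRevelation, then raises the Gold amount in its own card info Resources by one.
; It writes that updated Info back into the player's PlayerSpecificCards and CurrentCards lists in server state, locating the entry by matching card class.
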(event EventBeginPlay)

(event Collision|EventActorBeginOverlap
  (params (OtherActor :type Actor%20Object%20Reference)))

(event EventTick
  (params (DeltaSeconds :type Float%20%28single-precision%29)))

(fn ConstructionScript
  (|CallParentFunction))

(fn OnCardUse
  (params (Player :type PC%20Gameplay%20Object%20Reference) (Server :type GM%20Gameplay%20Object%20Reference))
  (bind _state (Variables|/Game/Gameplay/System/Server/GM_Gameplay.GM_Gameplay_C|GetState Server))
  (|CallParentFunction Player Server)
  (Default|ActivateCRevelation Server)
  (Utilities|Increment)
  (Utilities|ApplyChangestoArray (Variables|/Game/Gameplay/System/Cards/Framework/CardInfoList.CardInfoList_C|GetList (.Value (Utilities|Map|Find (Variables|/Game/Gameplay/System/Server/GS_Gameplay.GS_Gameplay_C|GetPlayerSpecificCards _state) Player))))
  (Utilities|ApplyChangestoArray (Variables|/Game/Gameplay/System/Cards/Framework/CardInfoList.CardInfoList_C|GetList (.Value (Utilities|Map|Find (Variables|/Game/Gameplay/System/Server/GS_Gameplay.GS_Gameplay_C|GetCurrentCards _state) Player)))))