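; Construction card base Blueprint that builds a structure when the card is used.
; On use it runs the parent card logic, then has the server build the card's Structure.
; If the player is a merchant, the server also adds a resource amount taken from the card's Gold value.
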(fn ConstructionScript
  (|CallParentFunction))

(fn OnCardUse
  (params (Player :type PC%20Gameplay%20Object%20Reference) (Server :type GM%20Gameplay%20Object%20Reference))
  (|CallParentFunction Player Server)
  (Default|BuildStructure Server (Variables|Default|GetStructure))
  (if (|IsPlayeraMerchant?)
    (Default|AddResource Server "NewEnumerator2" (.gold (Utilities|Struct|BreakCardInfo (Variables|Default|GetInfo))))))