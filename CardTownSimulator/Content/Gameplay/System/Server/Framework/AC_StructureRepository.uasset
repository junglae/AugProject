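; Server framework component that stores the level's roads, markets, farmlands and lumbermills and hands out random, unrepeated structures by type.
; Initialize clears the selection history and caches every actor of those four classes.
; GetRandomStructure picks from the array matching the type and records it in Selected.
; An already selected pick goes through a loop counter macro that checks a 100-iteration threshold to choose between retrying and returning.
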(event Custom|Initialize
  (Utilities|Array|Clear (Variables|Default|GetSelected))
  (bind _outactors (Actor|GetAllActorsOfClass "/Game/Gameplay/Client/Design/BP_Road.BP_Road_C"))
  (Variables|Default|SetRoads _outactors)
  (bind _outactors_2 (Actor|GetAllActorsOfClass "/Game/Gameplay/Client/Design/BP_Market.BP_Market_C"))
  (Variables|Default|SetMarkets _outactors_2)
  (bind _outactors_3 (Actor|GetAllActorsOfClass "/Game/Gameplay/Client/Design/BP_FarmLand.BP_FarmLand_C"))
  (Variables|Default|SetFarmlands _outactors_3)
  (bind _outactors_4 (Actor|GetAllActorsOfClass "/Game/Gameplay/Client/Design/BP_Lumbermill.BP_Lumbermill_C"))
  (Variables|Default|SetLumbermills _outactors_4))

(fn GetRandomStructure
  (params (Type :type EStructureType%20Enum :default "NewEnumerator0"))
  (LocalVariables|Setloop 0)
  (bind _output_get (LocalVariables|SetRandomActor (.OutItem (Utilities|Array|Random (Utilities|Select :Index Type :NewEnumerator0 (Variables|Default|GetRoads) :NewEnumerator1 (Variables|Default|GetMarkets) :NewEnumerator2 (Variables|Default|GetFarmlands) :NewEnumerator3 (Variables|Default|GetLumbermills)))) :!label _label))
  (if (Utilities|Array|ContainsItem (Variables|Default|GetSelected) _output_get)
    (|Loopcounter
      (:then
        (goto _label))
      (:Nope
        (return 0)))
    (else
      (Utilities|Array|Add (Variables|Default|GetSelected) (LocalVariables|GetRandomActor))
      (return (LocalVariables|GetRandomActor)))))