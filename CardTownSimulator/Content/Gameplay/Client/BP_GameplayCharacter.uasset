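; Gameplay character Blueprint with a zoomable spring-arm camera and a cosmetic hat and tool.
; BeginPlay socket-attaches a random hat to the head and a tool to the right hand, indexed by the hat function's unwired return rather than the random number.
; ZoomCamera steps a clamped Zoom value; Tick eases arm length toward a formula-derived target.
; Job, resource, building and delivery-animation functions are empty stubs.
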(event Custom|Zoom%20Camera
  (params (Zoom%20In :type Boolean))
  (Variables|Default|SetZoom (|(clamp(({4048459A-4497-95BD-A5ED-8EA7E000A083}+value),0,2)) (Math|Float|SelectFloat -0.1 0.1 Zoom%20In))))

(event Custom|Set%20Job%20Charator
  (params (JobInfo :type Card%20Info%20Structure)))

(event EventTick
  (params (DeltaSeconds :type Float%20%28single-precision%29))
  (|LerpCameraZoom)
  (if (|({4048459A-4497-95BD-A5ED-8EA7E000A083}<=1))
    (Transformation|AddLocalOffset (Variables|Camera|GetSpringArm) "0, 0, 0" false false)))

(event EventBeginPlay
  (bind _outnum (CallFunction|SetSkeletalMesh (Math|Random|RandomInteger 5)))
  (CallFunction|SetStaticMesh _outnum))

(fn ConstructionScript)

(fn SetSkeletalMesh
  (params (InNum :type Integer))
  (Components|SkeletalMesh|SetSkeletalMeshAsset (Variables|Default|GetSKM_Hat) (Utilities|Array|Get(acopy) (Variables|Default|GetSKMHatArray) InNum))
  (Transformation|AttachComponentToComponent (Variables|Default|GetSKM_Hat) (Variables|Default|GetSkeletalMesh) "headSocket" "KeepRelative" "KeepRelative" "KeepRelative" true))

(fn SetStaticMesh
  (params (InNum :type Integer))
  (Components|StaticMesh|SetStaticMesh (Variables|Default|GetTool) (Utilities|Array|Get(acopy) (Variables|Default|GetSKMStaticMesh) InNum))
  (Transformation|AttachComponentToComponent (Variables|Default|GetTool) (Variables|Default|GetSkeletalMesh) "hand_rSocket" "KeepRelative" "KeepRelative" "KeepRelative" true))

(fn CheckResource
  (params (NewParam1 :type E_ResourceType%20Enum :default "NewEnumerator5"))
  (return false 0))

(fn GetCurrentResources
  (return "NewEnumerator5"))

(fn PlayDeliverAnim
  (return 0.0))

(fn ProgressBuilding
  (params (Invested%20Time :type Float%20%28double-precision%29))
  (return 0.0))

(fn RemoveResource
  (return "NewEnumerator5" 0))