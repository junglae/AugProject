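; BPC_AIController is an AI controller that picks behavior trees and targets for its AI character.
; It runs BT_MainIdle on begin play, and ChangeStateActor maps the Idle or Build state to a DT_AIState row whose behavior tree it runs.
; TargetIn writes a given actor and its current location to Blackboard keys.
; The perception update handler, TargetActor and ChangeState are empty stubs.
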(event OnTargetPerceptionUpdated(AIPerception)
  (params (Actor :type Actor%20Object%20Reference) (Stimulus :type AI%20Stimulus%20Structure)))

(event Custom|TargetIn
  (params (InActor :type Actor%20Object%20Reference))
  (Variables|Default|SetInActor InActor)
  (AI|Components|Blackboard|SetValueasObject (Variables|Default|GetBlackboard) (Variables|Default|GetKeyName_Target) (Variables|Default|GetInActor))
  (AI|Components|Blackboard|SetValueasVector (Variables|Default|GetBlackboard) (Variables|Default|GetKeyName_TargetLocation) (Transformation|GetActorLocation (Variables|Default|GetInActor))))

(event Custom|ChangeStateActor
  (params (OutState :type EAIState%20Enum :default "NewEnumerator1"))
  (bind _returnvalue (Utilities|GetDataTableRow "/Game/Gameplay/Client/Blueprint/AI/Charactor/DT_AIState.DT_AIState" (Utilities|Select :Index OutState :NewEnumerator0 "Idle" :NewEnumerator1 "Build"))
    (:then
      (AI|RunBehaviorTree (.Behaivor (Utilities|Struct|BreakBPS_AIState _returnvalue))))))

(event EventBeginPlay
  (AI|RunBehaviorTree "/Game/Gameplay/Client/Blueprint/AI/Behaior/BT_MainIdle.BT_MainIdle"))

(fn ConstructionScript)

(fn TargetActor
  (params (InActor :type Actor%20Object%20Reference))
  (return 0))

(fn ChangeState
  (params (InAIState :type EAIState%20Enum :default "NewEnumerator0")))