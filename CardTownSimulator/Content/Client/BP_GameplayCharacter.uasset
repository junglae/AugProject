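; Gameplay character Blueprint that provides a smoothed, stepped camera zoom on a spring arm.
; ZoomCamera nudges a clamped Zoom value in or out through math expression nodes.
; Each Tick lerps the arm length halfway toward a target derived from Zoom, using a Floor term to steepen pull-back beyond 1.
; Tick also applies a zero, effectively no-op, spring arm offset under a zoom-threshold check.
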(event Custom|Zoom%20Camera
  (params (Zoom%20In :type Boolean))
  (Variables|Default|SetZoom (|(clamp(({4048459A-4497-95BD-A5ED-8EA7E000A083}+value),0,2)) (Math|Float|SelectFloat -0.1 0.1 Zoom%20In))))

(event EventTick
  (params (DeltaSeconds :type Float%20%28single-precision%29))
  (|LerpCameraZoom)
  (if (|({4048459A-4497-95BD-A5ED-8EA7E000A083}<=1))
    (Transformation|AddLocalOffset (Variables|Camera|GetSpringArm) "0, 0, 0" false false)))

(fn ConstructionScript)